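; BP_SpaceTruck is a destructible space truck in the arcade shooter that awards score and galaxy points when killed.
; On Destroyed it always removes its indicator, but only explodes and pays rewards through BP_ArcadeShooterGameModeBase if Health is zero or below.
; It finds that game mode with GetAllActorsOfClass.
; Two events play the damage and destruction sounds at the truck's location.
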(event EventBeginPlay)

(event Collision|EventActorBeginOverlap
  (params (OtherActor :type Actor%20Object%20Reference)))

(event EventTick
  (params (DeltaSeconds :type Float%20%28single-precision%29)))

(event EventDestroyed
  (Class|Ship|DestroyIndicator)
  (if (<= (Variables|Default|GetHealth) 0.0)
    (Class|Ship|SpaceTruckExplode (Variables|Default|GetAngle))
    (bind _outactors (Actor|GetAllActorsOfClass "/Game/Blueprints/BP_ArcadeShooterGameModeBase.BP_ArcadeShooterGameModeBase_C"))
    (Class|ArcadeShooterGameModeBase|IncrementScore (Utilities|Array|Get(acopy) _outactors) (Variables|Default|GetScore))
    (Class|ArcadeShooterGameModeBase|IncrementGalaxyPoints (Utilities|Array|Get(acopy) _outactors) (Variables|Default|GetGalaxyPoints))))

(event EventPlayDamageTakenSound
  (Audio|PlaySoundatLocation "/Game/Audio/Impact2.Impact2" (Transformation|GetActorLocation) "0, 0, 0" 1.0 1.0 0.0 0 0 0))

(event EventPlayDestroySound
  (Audio|PlaySoundatLocation "/Game/Audio/Explosion11.Explosion11" (Transformation|GetActorLocation) "0, 0, 0" 1.0 1.0 0.0 0 0 0))

(fn ConstructionScript)