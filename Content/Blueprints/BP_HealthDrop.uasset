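; Health drop pickup that supplies the pop-up feedback and chime sound for being collected.
; ShowPopUpMessage branches on FindBonuses: true spawns a +500 BP_PopUpMessage at the mesh and adds that score through the arcade shooter game mode.
; Otherwise it spawns a recoloured +1 pop-up without touching the score.
; The health change itself is not handled in this graph, and PlayPickUpSound only plays the chime at the actor's location.
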(event EventBeginPlay)

(event Collision|EventActorBeginOverlap
  (params (OtherActor :type Actor%20Object%20Reference)))

(event EventTick
  (params (DeltaSeconds :type Float%20%28single-precision%29)))

(event EventShowPopUpMessage
  (bind _meshcomponent (Variables|Default|GetMeshComponent))
  (bind _returnvalue (Transformation|GetWorldLocation _meshcomponent))
  (bind _returnvalue_2 (Class|Drop|FindBonuses true))
  (if _returnvalue_2
    (bind _returnvalue_3 (Game|SpawnActorfromClass "/Game/Blueprints/BP_PopUpMessage.BP_PopUpMessage_C" (Math|Transform|MakeTransform _returnvalue "0,180.000000, 0" "1,1,1") "Undefined" 0 0))
    (Rendering|Components|TextRender|SetText (Variables|/Game/Blueprints/BP_PopUpMessage.BP_PopUpMessage_C|GetMainText _returnvalue_3) (Utilities|Text|ToText(String) (Utilities|String|Append "+" "500")))
    (bind _outactors (Actor|GetAllActorsOfClass "/Game/Blueprints/BP_ArcadeShooterGameModeBase.BP_ArcadeShooterGameModeBase_C"))
    (Class|ArcadeShooterGameModeBase|IncrementScore (Utilities|Array|Get(acopy) _outactors) 500)
    (else
      (bind _returnvalue_4 (Game|SpawnActorfromClass "/Game/Blueprints/BP_PopUpMessage.BP_PopUpMessage_C" (Math|Transform|MakeTransform _returnvalue "0,180.000000, 0" "1,1,1") "Undefined" 0 0))
      (Rendering|Components|TextRender|SetText (Variables|/Game/Blueprints/BP_PopUpMessage.BP_PopUpMessage_C|GetMainText _returnvalue_4) (Utilities|Text|ToText(String) (Utilities|String|Append "+" "1")))
      (Rendering|Components|TextRender|SetTextRenderColor (Variables|/Game/Blueprints/BP_PopUpMessage.BP_PopUpMessage_C|GetMainText _returnvalue_4) (Math|Color|MakeColor 0 113 22 0)))))

(event EventPlayPickUpSound
  (Audio|PlaySoundatLocation "/Game/Audio/zapsplat_multimedia_game_sound_chime_mallet_warm_family_game_001_63138.zapsplat_multimedia_game_sound_chime_mallet_warm_family_game_001_63138" (Transformation|GetActorLocation) "0, 0, 0" 1.0 1.0 0.0 0 0 0))

(fn ConstructionScript)