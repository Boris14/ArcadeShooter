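; BP_RadialWeaponDrop is a radial weapon drop actor that handles a bonus Galaxy Points pop-up.
; ShowPopUpMessage finds the player ship and, if its ShouldShowBonusGP flag is set, clears the flag and spawns a BP_PopUpMessage at the drop's mesh.
; The pop-up shows the bonus amount, and the game mode adds the same points.
; The Blueprint itself contains no pickup or weapon logic.
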(event EventBeginPlay)

(event Collision|EventActorBeginOverlap
  (params (OtherActor :type Actor%20Object%20Reference)))

(event EventTick
  (params (DeltaSeconds :type Float%20%28single-precision%29)))

(event EventShowPopUpMessage
  (bind _outactors (Actor|GetAllActorsOfClass "/Game/Blueprints/BP_PlayerShip.BP_PlayerShip_C"))
  (Utilities|IsValid (Utilities|Array|Get(acopy) _outactors)
    (:Is%20Valid
      (if (Variables|/Script/ArcadeShooter.Ship|GetbShouldShowBonusGP (Utilities|Array|Get(acopy) _outactors))
        (Variables|/Script/ArcadeShooter.Ship|SetbShouldShowBonusGP (Utilities|Array|Get(acopy) _outactors) false)
        (bind _returnvalue (Game|SpawnActorfromClass "/Game/Blueprints/BP_PopUpMessage.BP_PopUpMessage_C" (Math|Transform|MakeTransform (Transformation|GetWorldLocation (Variables|Default|GetMeshComponent)) "0,180.000000, 0" "1,1,1") "Undefined" 0 0))
        (Rendering|Components|TextRender|SetText (Variables|/Game/Blueprints/BP_PopUpMessage.BP_PopUpMessage_C|GetSecondaryText _returnvalue) (Utilities|Text|ToText(String) (Utilities|String|Append "+" "50")))
        (bind _outactors_2 (Actor|GetAllActorsOfClass "/Game/Blueprints/BP_ArcadeShooterGameModeBase.BP_ArcadeShooterGameModeBase_C"))
        (Class|ArcadeShooterGameModeBase|IncrementGalaxyPoints (Utilities|Array|Get(acopy) _outactors_2) 50)))))

(fn ConstructionScript)