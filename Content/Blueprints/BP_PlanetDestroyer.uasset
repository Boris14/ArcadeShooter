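; Planet Destroyer boss for an arcade shooter, providing audio, particle effects and UI for the boss and its parts, with IsBody marking the body.
; Only the body creates the boss health bar on BeginPlay.
; Event hooks play sounds and spawn explosion or charge emitters, with charge variants chosen by Rage.
; On destruction it removes its indicator and, if Health is depleted, awards score and galaxy points through the game mode.
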(event EventPlayChargingSound
  (bind _returnvalue (Transformation|GetActorLocation))
  (if (and (== (Variables|Default|GetRage) 1) (Variables|Default|GetbIsBody))
    (Audio|PlaySoundatLocation "/Game/Audio/ChargingSoundRage1.ChargingSoundRage1" _returnvalue "0, 0, 0" 1.0 1.0 0.0 0 0 0)
    (else
      (Audio|PlaySoundatLocation "/Game/Audio/ChargingSoundRage2.ChargingSoundRage2" _returnvalue "0, 0, 0" 1.0 1.0 0.0 0 0 0))))

(event Collision|EventActorBeginOverlap
  (params (OtherActor :type Actor%20Object%20Reference)))

(event EventShowExplosion
  (params (ExplosionLocation :type Vector :default "0, 0, 0"))
  (Effects|SpawnEmitteratLocation "/Game/StarterContent/Particles/P_Explosion.P_Explosion" ExplosionLocation (Transformation|GetActorRotation)))

(event EventShowSpawnCharge
  (params (SpawnLocation :type Vector :default "0, 0, 0"))
  (if (== (Variables|Default|GetRage) 1)
    (Effects|SpawnEmitteratLocation "/Game/StarterContent/Particles/SpawnCharge1.SpawnCharge1" SpawnLocation)
    (else
      (Effects|SpawnEmitteratLocation "/Game/StarterContent/Particles/SpawnCharge2.SpawnCharge2" SpawnLocation))))

(event EventTick
  (params (DeltaSeconds :type Float%20%28single-precision%29)))

(event EventDestroyed
  (Class|Ship|DestroyIndicator)
  (if (<= (Variables|Default|GetHealth) 0.0)
    (bind _outactors (Actor|GetAllActorsOfClass "/Game/Blueprints/BP_ArcadeShooterGameModeBase.BP_ArcadeShooterGameModeBase_C"))
    (Class|ArcadeShooterGameModeBase|IncrementScore (Utilities|Array|Get(acopy) _outactors) (Variables|Default|GetScore))
    (Class|ArcadeShooterGameModeBase|IncrementGalaxyPoints (Utilities|Array|Get(acopy) _outactors) (Variables|Default|GetGalaxyPoints))))

(event EventPlayDamageTakenSound
  (Audio|PlaySoundatLocation "/Game/Audio/Impact2.Impact2" (Transformation|GetActorLocation) "0, 0, 0" 1.0 1.0 0.0 0 0 0))

(event EventPlayDestroySound
  (Audio|PlaySoundatLocation "/Game/Audio/Explosion11.Explosion11" (Transformation|GetActorLocation) "0, 0, 0" 1.0 1.0 0.0 0 0 0))

(event EventPlaySpawnSound
  (Audio|PlaySoundatLocation "/Game/Audio/SciFiGun11.SciFiGun11" (Transformation|GetActorLocation) "0, 0, 0" 1.0 1.0 0.0 0 0 0))

(event EventPlayDetachSound
  (Audio|PlaySoundatLocation "/Game/Audio/Detach.Detach" (Transformation|GetActorLocation) "0, 0, 0" 1.0 1.0 0.0 0 0 0))

(event EventBeginPlay
  (if (Variables|Default|GetbIsBody)
    (bind _returnvalue (UserInterface|CreateWidget "/Game/Blueprints/BP_BossHealthBar.BP_BossHealthBar_C"))
    (UserInterface|Viewport|AddtoViewport _returnvalue 0)))

(event EventShowShootingCharge
  (params (SpawnLocation :type Vector :default "0, 0, 0"))
  (if (== (Variables|Default|GetRage) 1)
    (Effects|SpawnEmitteratLocation "/Game/StarterContent/Particles/ShootCharge1.ShootCharge1" SpawnLocation)
    (else
      (Effects|SpawnEmitteratLocation "/Game/StarterContent/Particles/ShootCharge2.ShootCharge2" SpawnLocation))))

(fn ConstructionScript)