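; BP_SpaceTruckParticle is an arcade shooter actor, named for a space truck, that pays out rewards when destroyed with no health left.
; On Destroyed, if Health is zero or below, it adds Score to the game mode and awards a tenth of it to the player ship as galaxy points.
; It finds both targets with GetAllActorsOfClass, using the first result without a validity check.
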(event EventBeginPlay)

(event Collision|EventActorBeginOverlap
  (params (OtherActor :type Actor%20Object%20Reference)))

(event EventTick
  (params (DeltaSeconds :type Float%20%28single-precision%29)))

(event EventDestroyed
  (if (<= (Variables|Default|GetHealth) 0.0)
    (bind _outactors (Actor|GetAllActorsOfClass "/Game/Blueprints/BP_ArcadeShooterGameModeBase.BP_ArcadeShooterGameModeBase_C"))
    (Class|ArcadeShooterGameModeBase|IncrementScore (Utilities|Array|Get(acopy) _outactors) (Variables|Default|GetScore))
    (bind _outactors_2 (Actor|GetAllActorsOfClass "/Game/Blueprints/BP_PlayerShip.BP_PlayerShip_C"))
    (Class|Ship|AcquireGalaxyPoints (Utilities|Array|Get(acopy) _outactors_2) (/ (Variables|Default|GetScore) 1e+01))))

(fn ConstructionScript)